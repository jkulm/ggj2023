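; Rain spawner actor that drops collectable droplets from a pre-spawned object pool.
; On BeginPlay it spawns the pool at random points in a shell between inner and outer sphere radii, sized in the construction script.
; If Raining is set, a looping timer releases batches of droplets by enabling physics.
; ReturnObjectToPool stops a droplet's physics, resets its scale, teleports it back into the shell and re-adds it.
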(event `self.ReceiveBeginPlay`
  (`self._SpawnPool`)
  (if (`self.bRaining`)
    (`KismetSystemLibrary.K2_SetTimer` null "_Rain" 2.0 true 4.0)))

(fn `_DropPooledDroplet`
  (if (> (`KismetArrayLibrary.Array_Length` (`self.RaindropPool`)) 0)
    (bind _output_get (set `self.PooledObject` (`|GetArrayItem` (`self.RaindropPool`))))
    (`KismetArrayLibrary.Array_RemoveItem` (`self.RaindropPool`) _output_get)
    (`PrimitiveComponent.SetSimulatePhysics` (`/Game/Characters/BP_CollectableDroplets.StaticMesh` (`self.PooledObject`)) true)))

(fn `_Rain`
  (for _ (range (+ (`KismetMathLibrary.Clamp` (`self.ConstantRainCount`) 0 (`KismetArrayLibrary.Array_Length` (`self.RaindropPool`))) 1))
    (`self._DropPooledDroplet`)))

(fn `_SpawnPool`
  (for _index (range (`self.MaxPoolSize`))
    (bind _returnvalue (`|SpawnActorFromClass` "/Game/Characters/BP_CollectableDroplets.BP_CollectableDroplets_C" (`KismetMathLibrary.MakeTransform` (+ (`self.K2_GetActorLocation`) (* (`KismetMathLibrary.RandomUnitVector`) (`KismetMathLibrary.RandomFloatInRange` (`self.DropSphereInnerRadius`) (`self.DropSphereOuterRadius`))))) "Undefined" "OverrideRootScale" self _index null))
    (`KismetArrayLibrary.Array_Add` (`self.RaindropPool`) _returnvalue)))

(fn `ReturnObjectToPool`
  (params (ReturnObject :type "/Game/Characters/BP_CollectableDroplets Object Reference"))
  (bind _output_get (set `self.ReturnObject` ReturnObject))
  (`PrimitiveComponent.SetSimulatePhysics` (`/Game/Characters/BP_CollectableDroplets.StaticMesh` (`self.ReturnObject`)) false)
  (`self.SetActorScale3D` (`self.ReturnObject`) (1.0 1.0 1.0))
  (`self.K2_TeleportTo` :`self` (`self.ReturnObject`) :`DestLocation` (+ (`self.K2_GetActorLocation`) (* (`KismetMathLibrary.RandomUnitVector`) (`KismetMathLibrary.RandomFloatInRange` (`self.DropSphereInnerRadius`) (`self.DropSphereOuterRadius`)))))
  (`KismetArrayLibrary.Array_Add` (`self.RaindropPool`) (`self.ReturnObject`)))

(fn `UserConstructionScript`
  (`SphereComponent.SetSphereRadius` (`self.OuterSpawnRadius`) (`self.DropSphereOuterRadius`) true)
  (`SphereComponent.SetSphereRadius` (`self.InnerSpawnRadius`) (`self.DropSphereInnerRadius`) true))