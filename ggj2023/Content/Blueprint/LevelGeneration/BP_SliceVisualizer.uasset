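; BP_SliceVisualizer is a level-generation debug actor that draws the bounds of a slice as a cylinder.
; The cylinder rises from the root component's height by SliceHeight, with a radius of half SliceBounds, and persists through a very long duration.
; The construction script draws it when DebugBounds is set, otherwise flushes all persistent debug lines.
; BeginPlay flushes first, then repeats that logic after a short delay.
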(event `self.ReceiveBeginPlay`
  (bind (_returnvalue_x _returnvalue_y _returnvalue_z) (`KismetMathLibrary.BreakVector` (`SceneComponent.K2_GetComponentLocation` (`self.DefaultSceneRoot`))))
  (`KismetSystemLibrary.FlushPersistentDebugLines`)
  (`KismetSystemLibrary.Delay` 0.8)
  (if (`self.DebugBounds`)
    (`KismetSystemLibrary.DrawDebugCylinder` (`KismetMathLibrary.MakeVector` 0.0 0.0 _returnvalue_z) (`KismetMathLibrary.MakeVector` 0.0 0.0 (+ (`self.SliceHeight`) _returnvalue_z)) (* (`self.SliceBounds`) 0.5) 16 (`self.Color`) 1e+21 20.0)
    (else
      (`KismetSystemLibrary.FlushPersistentDebugLines`))))

(fn `UserConstructionScript`
  (bind (_returnvalue_x _returnvalue_y _returnvalue_z) (`KismetMathLibrary.BreakVector` (`SceneComponent.K2_GetComponentLocation` (`self.DefaultSceneRoot`))))
  (if (`self.DebugBounds`)
    (`KismetSystemLibrary.DrawDebugCylinder` (`KismetMathLibrary.MakeVector` 0.0 0.0 _returnvalue_z) (`KismetMathLibrary.MakeVector` 0.0 0.0 (+ (`self.SliceHeight`) _returnvalue_z)) (* (`self.SliceBounds`) 0.5) 16 (`self.Color`) 1e+21 20.0)
    (else
      (`KismetSystemLibrary.FlushPersistentDebugLines`))))