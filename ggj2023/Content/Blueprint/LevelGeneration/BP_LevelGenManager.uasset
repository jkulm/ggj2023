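; Level generator that builds a vertical stack of slice actors at BeginPlay, from roots at the base to clouds on top.
; Between them it spawns runs of empty, branch and canopy slices, with counts from variables and branch and canopy classes picked randomly from lists.
; SpawnLoop spawns each run, advancing NextSpawnHeight by each slice's SliceHeight so the next sits above it.
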(event `self.ReceiveBeginPlay`
  ;[1 1 1] Roots at base layer
  (bind _returnvalue (`|SpawnActorFromClass` "/Game/Blueprint/LevelGeneration/LevelSlices/BP_Slice_Roots.BP_Slice_Roots_C" (`KismetMathLibrary.MakeTransform` (0.0 0.0 0.0)) "AlwaysSpawn" "OverrideRootScale" null null))
  (set `self.NextSpawnHeight` (`/Game/Blueprint/LevelGeneration/LevelSlices/BP_MasterSlice.SliceHeight` _returnvalue))
  (`self.SpawnLoop` (`self.EmptyBeforeRoots`) "/Game/Blueprint/LevelGeneration/LevelSlices/BP_Slice_Empty.BP_Slice_Empty_C")
  (`self.SpawnLoop` (`self.Branch2`) (`KismetArrayLibrary.Array_Random` (`self.BranchSliceList`)))
  (`self.SpawnLoop` (`self.EmptyBetweenBranches`) "/Game/Blueprint/LevelGeneration/LevelSlices/BP_Slice_Empty.BP_Slice_Empty_C")
  (`self.SpawnLoop` (`self.Branch1`) (`KismetArrayLibrary.Array_Random` (`self.BranchSliceList`)))
  (`self.SpawnLoop` (`self.EmptyBeforeCanopy`) (`KismetArrayLibrary.Array_Random` (`self.CanopySliceList`)))
  (`|SpawnActorFromClass` "/Game/Blueprint/LevelGeneration/LevelSlices/BP_Slice_Clouds.BP_Slice_Clouds_C" (`KismetMathLibrary.MakeTransform` (`KismetMathLibrary.MakeVector` 0.0 0.0 (`self.NextSpawnHeight`))) "AlwaysSpawn" "OverrideRootScale" null null))

(fn `SpawnLoop`
  (params (Number :type Integer) (Actor :type "Actor Class Reference"))
  (for _ (range (+ (`KismetMathLibrary.Clamp` (- Number 1) 0 100) 1))
    (bind _returnvalue (`|SpawnActorFromClass` Actor (`KismetMathLibrary.MakeTransform` (`KismetMathLibrary.MakeVector` 0.0 0.0 (`self.NextSpawnHeight`))) "AlwaysSpawn" "OverrideRootScale" null null))
    (bind _asbp_master_slice (cast `/Game/Blueprint/LevelGeneration/LevelSlices/BP_MasterSlice` _returnvalue))
    (set `self.NextSpawnHeight` (+ (`self.NextSpawnHeight`) (`/Game/Blueprint/LevelGeneration/LevelSlices/BP_MasterSlice.SliceHeight` _asbp_master_slice))))
  (return))

(fn `UserConstructionScript`)