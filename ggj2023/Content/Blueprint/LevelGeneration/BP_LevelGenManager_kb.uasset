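; Level generation manager that builds a vertical tree level at BeginPlay by stacking randomly chosen sublevel slices.
; LoadSliceLoop creates streaming level instances at a running NextSpawnHeight, stacking empty tree, branch, canopy, canopy top, empty and cloud sections in order.
; Each slice advances the height by SliceHeight or an override, and WinddownHeight records where branches begin.
; An actor-based SpawnLoop is defined but not called here, and debug lines can be flushed after a delay.
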(event `self.ReceiveBeginPlay`
  (`|ExecutionSequence`
    (:`then_0`
      (set `self.NextSpawnHeight` (`self.RootSliceHeight`))
      (`self.LoadSliceLoop` (`self.EmptyBeforeRoots`) (`self.EmptyTreeLevelList`))
      (set `self.WinddownHeight` (`self.NextSpawnHeight`))
      (`self.LoadSliceLoop` (`self.Branch1`) (`self.BranchLevelList`))
      (`self.LoadSliceLoop` (`self.Canopy`) (`self.CanopyLevelList`))
      (`self.LoadSliceLoop` 1 (`self.CanopyTopLevelList`) true (`self.CanopyTopSliceHeight`))
      (`self.LoadSliceLoop` (`self.EmptyBeforeCanopy`) (`self.EmptyLevelList`))
      (`self.LoadSliceLoop` 1 (`self.CloudLevelList`)))
    (:`then_1`
      (if (`self.ClearSliceDebug`)
        (`KismetSystemLibrary.Delay` 1.0)
        (`KismetSystemLibrary.FlushPersistentDebugLines`)))))

(fn `LoadSliceLoop`
  (params (Number :type Integer) (LevelNames :type "Array of Name") (OverrideSliceHeight :type Boolean) (OverrideHeightValue :type "Float (double-precision)"))
  (bind _output (`|GetArrayItem` LevelNames (`KismetMathLibrary.RandomInteger` (`KismetArrayLibrary.Array_Length` LevelNames))))
  (for _index (range (+ (`KismetMathLibrary.Clamp` (- Number 1) 0 100) 1))
    (bind _returnvalue (`LevelStreaming.CreateInstance` (`GameplayStatics.GetStreamingLevel` _output) (`KismetStringLibrary.Concat_StrStr` (`KismetStringLibrary.Conv_NameToString` _output) "_" (`KismetStringLibrary.Conv_IntToString` _index))))
    (set `LevelStreaming.LevelTransform` (`KismetMathLibrary.MakeTransform` (`KismetMathLibrary.MakeVector` 0.0 0.0 (`self.NextSpawnHeight`))) _returnvalue)
    (set `LevelStreaming.bShouldBeLoaded` true _returnvalue)
    (set `LevelStreaming.bShouldBeVisible` true _returnvalue)
    (if OverrideSliceHeight
      (set `self.NextSpawnHeight` (+ (`self.NextSpawnHeight`) OverrideHeightValue))
      (else
        (set `self.NextSpawnHeight` (+ (`self.NextSpawnHeight`) (`self.SliceHeight`))))))
  (return))

(fn `SpawnLoop`
  (params (Number :type Integer) (Actor :type "Actor Class Reference"))
  (for _ (range (+ (`KismetMathLibrary.Clamp` (- Number 1) 0 100) 1))
    (bind _returnvalue (`|SpawnActorFromClass` Actor (`KismetMathLibrary.MakeTransform` (`KismetMathLibrary.MakeVector` 0.0 0.0 (`self.NextSpawnHeight`))) "AlwaysSpawn" "OverrideRootScale" null null))
    (bind _asbp_master_slice (cast `/Game/Blueprint/LevelGeneration/LevelSlices/BP_MasterSlice` _returnvalue))
    (set `self.NextSpawnHeight` (+ (`self.NextSpawnHeight`) (`/Game/Blueprint/LevelGeneration/LevelSlices/BP_MasterSlice.SliceHeight` _asbp_master_slice))))
  (return))

(fn `UserConstructionScript`)