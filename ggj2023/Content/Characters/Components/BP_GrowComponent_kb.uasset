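; Actor component that grows its owner when it absorbs droplets and shrinks it when it takes point damage.
; Overlaps and hits with collectable droplets add scale and return them to their pool; damage subtracts scale, applies knockback inversely proportional to scale and starts timed invulnerability.
; Clamped scale resizes BP_HERO's sphere and capsule, or any other owner's whole actor.
; Reaching minimum scale fires AllDriedUp.
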(event `self.ReceiveBeginPlay`
  (bind _asbp_hero (cast `/Game/Developers/KavanBahrami/Core/BP_HERO` (`self.GetOwner`))
    (:`then`
      (bind _output_get (set `self.As BP HERO` _asbp_hero))
      (set `self.InitialOwnerScale` (`SceneComponent.RelativeScale3D` (`/Game/Developers/KavanBahrami/Core/BP_HERO.Sphere` _output_get)))
      (set `self.InitialCapsuleRadius` (`CapsuleComponent.CapsuleRadius` (`Character.CapsuleComponent` _output_get))))
    (:`CastFailed`
      (set `self.InitialOwnerScale` (`Actor.GetActorScale3D` (`self.GetOwner`)))))
  (add `Actor.OnActorBeginOverlap` (`self.GetOwner`) (delegate `Overlap`))
  (add `Actor.OnActorHit` (`self.GetOwner`) (delegate `OnActorHit_Event`))
  ;[0.01938 0.01938 0.01938] Damage Event
  (add `Actor.OnTakePointDamage` (`self.GetOwner`) (delegate `OnTakePointDamage_Event`)))

(event `Overlap`
  (params (OverlappedActor :type "Actor Object Reference") (OtherActor :type "Actor Object Reference"))
  (`self.OnOverlap` OverlappedActor OtherActor))

(event `OnActorHit_Event`
  (params (SelfActor :type "Actor Object Reference") (OtherActor :type "Actor Object Reference") (NormalImpulse :type "Vector Structure") (Hit :type "HitResult Structure (by ref)"))
  (`self.OnOverlap` SelfActor OtherActor))

(event `OnTakePointDamage_Event`
  (params (DamagedActor :type "Actor Object Reference") (Damage :type "Float (single-precision)") (InstigatedBy :type "Controller Object Reference") (HitLocation :type "Vector Structure") (FHitComponent :type "PrimitiveComponent Object Reference") (BoneName :type Name) (ShotFromDirection :type "Vector Structure") (DamageType :type "DamageType Object Reference") (DamageCauser :type "Actor Object Reference"))
  ;[0.01938 0.01938 0.01938] Damage Event
  (if (`self.DEBUG`)
    (`KismetSystemLibrary.PrintString` "e Take Damage"))
  (if (not (`self.IsInvulnerable`))
    (set `self.IsInvulnerable` true)
    (`/Engine/EditorBlueprintResources/StandardMacros.IncrementInt` (`self.HitsReceived`)
      (:`  `
        (`KismetSystemLibrary.K2_SetTimerDelegate` (delegate `RemoveInvulnerability`) (`self.InvulnerabilityTime`))
        (if (== Damage 0.0)
          (`self.CaculateUpdatedScale` (* (`self.Increment`) -1.0))
          (else
            (`self.CaculateUpdatedScale` (* Damage -0.01))))
        (`self.UpdateOwnerScale`)
        (`self.ApplyKnockback` ShotFromDirection)))))

(event `RemoveInvulnerability`
  ;[0.01938 0.01938 0.01938] Damage Event
  (set `self.IsInvulnerable` false))

(fn `ApplyKnockback`
  (params (Direction :type "Vector Structure"))
  (bind _ascharacter (cast `Character` (`self.GetOwner`)))
  (if (`self.DEBUG`)
    (`KismetSystemLibrary.PrintString` "ApplyKnockBack"))
  (`CharacterMovementComponent.AddImpulse` (`Character.CharacterMovement` _ascharacter) (* Direction (/ (`self.KnockbackStrength`) (`self.Scale`)) -1.0) false))

(fn `CaculateUpdatedScale`
  (params (ScaleIncrease :type "Float (double-precision)"))
  (bind _output_get (set `self.Scale` (`KismetMathLibrary.FClamp` (+ ScaleIncrease (`self.Scale`)) (`self.MinScale`) (`self.MaxScale`))))
  (if (<= _output_get (`self.MinScale`))
    (`self.AllDriedUp` (`self.GetOwner`))))

(fn `OnOverlap`
  (params (SelfRef :type "Actor Object Reference") (OtherActor :type "Actor Object Reference"))
  (if (!= OtherActor (`self._LastInteract`))
    (set `self._LastInteract` (`local.OtherActor`))
    (if (`self.DEBUG`)
      (`KismetSystemLibrary.PrintString` (`KismetStringLibrary.Concat_StrStr` (`KismetSystemLibrary.GetDisplayName` (`local.SelfRef`)) " has collided with " (`KismetSystemLibrary.GetDisplayName` (`local.OtherActor`))) true true (struct :`G` 0.66 :`B` 1.0 :`A` 1.0) 1.0))
    (cast `/Game/Developers/KavanBahrami/Core/BP_CollectableDroplets` (`local.OtherActor`)
      (:`then`
        (`self.ObsorbedDroplet`)
        (`self.CaculateUpdatedScale` (`self.Increment`))
        (`self.UpdateOwnerScale`)
        (bind _asbp_collectable_droplets (cast `/Game/Developers/KavanBahrami/Core/BP_CollectableDroplets` (`local.SelfRef`))
          (:`then`
            (`/Engine/EditorBlueprintResources/StandardMacros.IncrementInt` (`self.DropletsAbsorbed`)
              (:`  `
                (message `/Game/Developers/KavanBahrami/Core/BPI_RainPool.ReturnToPool` (`local.OtherActor`) (`/Game/Developers/KavanBahrami/Core/BP_CollectableDroplets.DropIndex` _asbp_collectable_droplets)))))
          (:`CastFailed`
            (message `/Game/Developers/KavanBahrami/Core/BPI_RainPool.ReturnToPool` (`local.OtherActor`) 0))))
      (:`CastFailed`
        (if (`self.DEBUG`)
          (`KismetSystemLibrary.PrintString` (`KismetSystemLibrary.GetDisplayName` (`local.OtherActor`))))))))

(fn `UpdateOwnerScale`
  (bind _initialownerscale (`self.InitialOwnerScale`))
  (bind _scale (`self.Scale`))
  (bind _returnvalue (* (`self.InitialCapsuleRadius`) (`self.Scale`)))
  (bind _returnvalue_2 (* _initialownerscale _scale))
  (bind _capsulecomponent (`Character.CapsuleComponent` (`self.As BP HERO`)))
  (`self.As BP HERO`
    (:`then`
      (if (`self.DEBUG`)
        (`KismetSystemLibrary.PrintText` (`|FormatText` "HeroInitScale{InitialScale} - Scale{Scale} = NewScale{NewScale} ... UpdatedCapsuleSize = {CapsuleSize}" (`KismetStringLibrary.Conv_VectorToString` _initialownerscale) _scale (`KismetStringLibrary.Conv_VectorToString` _returnvalue_2) _returnvalue)))
      (`SceneComponent.SetRelativeScale3D` (`/Game/Developers/KavanBahrami/Core/BP_HERO.Sphere` (`self.As BP HERO`)) _returnvalue_2)
      (`CapsuleComponent.SetCapsuleHalfHeight` _capsulecomponent _returnvalue true)
      (`CapsuleComponent.SetCapsuleRadius` _capsulecomponent _returnvalue true))
    (:`else`
      (`Actor.SetActorScale3D` (`self.GetOwner`) (* (`self.InitialOwnerScale`) (`self.Scale`))))))