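; Actor component that slides its owner along spline objects it hits, keeping the owner's rotation.
; HitSomething queries the hit object for spline data, disables physics, sets Flying movement and starts a looping timer.
; Each tick samples a curve over elapsed time to position the owner along the spline, restarting if LockedToSpline.
; Otherwise ExitSlide fires a release event and delays re-attachment briefly; grinding code is unused test leftovers.
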(event `self.ReceiveBeginPlay`
  (set `self.ComponenetOwner` (`self.GetOwner`))
  (if (`self.bLockedToSpline`)
    (bind _currentsplineobject (`self.CurrentSplineObject`)
      (:`then`
        (`self.StartSlideTimer` _currentsplineobject))
      (:`else`
        (`KismetSystemLibrary.PrintString` "Error: Character set as Snapped to an unset Spline")))))

(event `StartSlideTimer`
  (params (_ActiveSplineObject :type "/Game/Developers/KavanBahrami/Core/Spline/BP_Spline Object Reference"))
  (`/Engine/EditorBlueprintResources/StandardMacros.IsValid` _ActiveSplineObject
    (:`Is Valid`
      (bind _returnvalue (`KismetSystemLibrary.K2_SetTimerDelegate` (delegate `SlidingLoop`) 0.01 true))
      (set `self.SlideTimer` _returnvalue))
    (:`Is Not Valid`
      (`KismetSystemLibrary.PrintString` "StartSlide passed INVALID Spline"))))

(event `SlidingLoop`
  (if (`self.bOnSpline`)
    ;[0.01938 0.01938 0.01938] Increment Time
    (bind _output_get (set `self.Time` (+ (`self.Time`) (`GameplayStatics.GetWorldDeltaSeconds`))))
    (bind _output_get_2 (set `self.Alpha` (`CurveFloat.GetFloatValue` (`self.Curve`) (+ (`self.StartOffset`) (* _output_get (/ 1.0 (`self.SplineDuration`)))))))
    (if (`KismetMathLibrary.NearlyEqual_FloatFloat` _output_get_2 1.0)
      (if (`self.bLockedToSpline`)
        (set `self.Time` 0.0)
        (set `self.StartOffset` 0.0)
        (else
          (`self.ExitSlide`)))
      (else
        (`self.Sliding` (stale `StartSlideTimer` _ActiveSplineObject) (`self.Alpha`))))))

(event `ExitSlide`
  (if (`self.bOnSpline`)
    (`self.SplineReleasedActor`)
    (`KismetSystemLibrary.K2_ClearAndInvalidateTimerHandle` (`self.SlideTimer`))
    (`KismetSystemLibrary.Delay` 0.2)
    (set `self.bOnSpline` false) ; Might need to delay this by a moment
  ))

(event `_StartGrinding`
  (params (Component :type "SceneComponent Object Reference") (Target :type "CapsuleComponent Object Reference") (Target2 :type "SceneComponent Object Reference"))
  (set `self.GrindSpeed` 1200.0))

(event `SlideAlongSpline`
  (params (SplineObject :type "/Game/Developers/KavanBahrami/Core/Spline/BP_Spline Object Reference"))
  (`/Engine/EditorBlueprintResources/StandardMacros.IsValid` SplineObject
    (:`Is Valid`
      (`KismetSystemLibrary.PrintString` "SlideAlong passed Valid Spline"))
    (:`Is Not Valid`
      (`KismetSystemLibrary.PrintString` "SlideAlong passed INVALID Spline"))))

(fn `HitSomething`
  (params (HitObject :type "Object Object Reference") (Hit :type "HitResult Structure (by ref)") (CharacterMovement :type "CharacterMovementComponent Object Reference") (TargetPrimitive :type "PrimitiveComponent Object Reference"))
  (set `self.SimulatingPrimitive` TargetPrimitive)
  (if (not (`self.bOnSpline`))
    (bind (_bslideable _bpsplineobjectref) (message `/Game/Developers/KavanBahrami/Core/Spline/BPI_SplineSlideObjects.CheckForSlideObject` HitObject))
    (if _bslideable
      ;[0 0 0] OtherDrops
      (`PrimitiveComponent.SetSimulatePhysics` (`self.SimulatingPrimitive`) false)
      (bind (_spline _splineduration _startpoint _direction _splinemeshoffset) (message `/Game/Developers/KavanBahrami/Core/Spline/BPI_SplineSlideObjects.GetSplineVariables` HitObject (`.ImpactPoint` (`GameplayStatics.BreakHitResult` Hit)) (`Actor.K2_GetActorLocation` (`self.ComponenetOwner`)) (`KismetMathLibrary.VSize` (`Actor.GetVelocity` (`self.ComponenetOwner`)))))
      (set `self.SplineMeshOffset` _splinemeshoffset)
      (set `self.SplineDuration` _splineduration) ; Setting the speed of each spline on the spline
      (bind _output_get (set `self.StartOffset` (/ _startpoint (`SplineComponent.GetSplineLength` _spline))))
      (set `self.bOnSpline` true)
      (`self.StartSlideTimer` _bpsplineobjectref)
      (bind _charactermovement (`local.CharacterMovement`)
        (:`then`
          (`CharacterMovementComponent.SetMovementMode` _charactermovement "MOVE_Flying" 0))
        (:`else`)))))

(fn `Sliding`
  (params (CurrentSplineObject :type "/Game/Developers/KavanBahrami/Core/Spline/BP_Spline Object Reference") (Alpha :type "Float (double-precision)"))
  (bind _spline (`/Game/Developers/KavanBahrami/Core/Spline/BP_Spline.Spline` CurrentSplineObject))
  (bind (_returnvalue_x _returnvalue_y _returnvalue_z) (`KismetMathLibrary.BreakVector` (`SplineComponent.GetLocationAtDistanceAlongSpline` _spline (`KismetMathLibrary.Lerp` 0.0 (`SplineComponent.GetSplineLength` _spline) Alpha) "World")))
  (`Actor.K2_SetActorLocationAndRotation` (`self.ComponenetOwner`) (`KismetMathLibrary.MakeVector` _returnvalue_x _returnvalue_y (+ _returnvalue_z (`self.SplineMeshOffset`))) (`Actor.K2_GetActorRotation` (`self.ComponenetOwner`)) false false)
  (return))

(fn `SplineReleasedActor`
  (`self.SplineReleasedActorEvent`))