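; Actor component that uses the owner's size as health, growing it when it overlaps droplets and shrinking it when it takes point damage.
; Droplet pickups are destroyed on overlap, while hits start a timed invulnerability window and apply an impulse to Character owners against the shot direction.
; Scale multiplies the initial actor scale, is capped at a maximum, and fires the OnKilled dispatcher below the minimum.
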(event `self.ReceiveBeginPlay`
  (bind _returnvalue (`self.GetOwner`))
  (set `self.InitialOwnerScale` (`Actor.GetActorScale3D` _returnvalue))
  (add `Actor.OnActorBeginOverlap` _returnvalue (delegate `OnActorBeginOverlap_Event`))
  (add `Actor.OnTakePointDamage` _returnvalue (delegate `OnTakePointDamage_Event`)))

(event `OnActorBeginOverlap_Event`
  (params (OverlappedActor :type "Actor Object Reference") (OtherActor :type "Actor Object Reference"))
  (cast `/Game/Environment/Powerups/BP_Droplet` OtherActor)
  (`self.IncreaseScale` (`self.Increment`))
  (`self.UpdateOwnerScale` OverlappedActor)
  (`Actor.K2_DestroyActor` OtherActor))

(event `OnTakePointDamage_Event`
  (params (DamagedActor :type "Actor Object Reference") (Damage :type "Float (single-precision)") (InstigatedBy :type "Controller Object Reference") (HitLocation :type "Vector Structure") (FHitComponent :type "PrimitiveComponent Object Reference") (BoneName :type Name) (ShotFromDirection :type "Vector Structure") (DamageType :type "DamageType Object Reference") (DamageCauser :type "Actor Object Reference"))
  (if (not (`self.IsInvulnerable`))
    (set `self.IsInvulnerable` true)
    (`KismetSystemLibrary.K2_SetTimerDelegate` (delegate `RemoveInvulnerability`) (`self.InvulnerabilityTime`))
    (if (== Damage 0.0)
      (`self.IncreaseScale` (* (`self.Increment`) -1.0))
      (else
        (`self.IncreaseScale` (* Damage -0.01))))
    (`self.UpdateOwnerScale` DamagedActor)
    (`self.ApplyKnockback` ShotFromDirection)))

(event `RemoveInvulnerability`
  (set `self.IsInvulnerable` false))

(fn `ApplyKnockback`
  (params (Direction :type "Vector Structure"))
  (bind _ascharacter (cast `Character` (`self.GetOwner`)))
  (`CharacterMovementComponent.AddImpulse` (`Character.CharacterMovement` _ascharacter) (* Direction (`self.KnockbackStrength`) -1.0) false))

(fn `IncreaseScale`
  (params (ScaleIncrease :type "Float (double-precision)"))
  (bind _maxscale (`self.MaxScale`))
  (bind _returnvalue (+ ScaleIncrease (`self.Scale`)))
  (if (< _returnvalue _maxscale)
    (bind _output_get (set `self.Scale` _returnvalue))
    (if (< _output_get (`self.MinScale`))
      (`self.OnKilled` (`self.GetOwner`)))
    (else
      (set `self.Scale` _maxscale))))

(fn `UpdateOwnerScale`
  (params (Target :type "Actor Object Reference"))
  (`Actor.SetActorScale3D` Target (* (`self.InitialOwnerScale`) (`self.Scale`))))