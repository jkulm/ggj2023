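; Camera controller component for BP_HERO that reframes the follow camera and plays shakes for falling, grinding, jumping, landing and speed changes.
; Movement events other than Jump pass targets to StartTransition, whose looping timer interpolates boom rotation, camera offset, rotation and FOV.
; Interpolation uses accumulated time as its delta, so it accelerates, and is held off early in game time to avoid snapping.
; A new shake class replaces the current shake, while duplicate requests are ignored.
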(event `self.ReceiveBeginPlay`
  (bind _asbp_hero (cast `/Game/Developers/KavanBahrami/Core/BP_HERO` (`self.GetOwner`))
    (:`then`
      (set `self._OwnerBoom` (`/Game/Developers/KavanBahrami/Core/BP_HERO.CameraBoom` _asbp_hero))
      (bind _output_get (set `self._OwnerCamera` (`/Game/Developers/KavanBahrami/Core/BP_HERO.FollowCamera` _asbp_hero)))
      (set `self._CameraDefaultFOV` (`CameraComponent.FieldOfView` _output_get)))
    (:`CastFailed`
      (`KismetSystemLibrary.PrintString` "Warning: CameraController expects HERO droplet"))))

(event `StartFalling`
  (`self.StartTransition` (struct :`Pitch` -60.0) (0.0 0.0 200.0) (struct :`Pitch` -30.0) (+ (`self._CameraDefaultFOV`) 10.0))
  (`self.StartCameraShake` "/Game/Developers/ShepherdDuff/CameraShake_Falling.CameraShake_Falling_C"))

(event `StartGrinding`
  (`self.StartTransition` (struct :`Pitch` -10.0) (0.0 0.0 0.0) (struct :`Pitch` 10.0) (`self._CameraDefaultFOV`))
  (`self.StartCameraShake` "/Game/Developers/ShepherdDuff/CameraShake_Land.CameraShake_Land_C"))

(event `Jump`
  (`self.StartCameraShake` "/Game/Developers/ShepherdDuff/CameraShake_Jump.CameraShake_Jump_C"))

(event `Land`
  (`self.StartTransition` (struct :`Pitch` -10.0) (0.0 0.0 0.0) (struct :`Pitch` 10.0) (`self._CameraDefaultFOV`))
  (`self.StartCameraShake` "/Game/Developers/ShepherdDuff/CameraShake_Land.CameraShake_Land_C"))

(event `SlowDown`
  (`self.StartTransition` (struct :`Pitch` -60.0) (150.0 0.0 250.0) (struct :`Pitch` -30.0) (`self._CameraDefaultFOV`))
  (`self.StartCameraShake` "/Game/Developers/ShepherdDuff/CameraShake_SlowDown.CameraShake_SlowDown_C"))

(event `SpeedUp`
  (`self.StartTransition` (struct :`Pitch` -60.0) (-150.0 0.0 250.0) (struct :`Pitch` -30.0) (+ (`self._CameraDefaultFOV`) 15.0))
  (`self.StartCameraShake` "/Game/Developers/ShepherdDuff/CameraShake_SpeedUp.CameraShake_SpeedUp_C"))

(event `StartTransition`
  (params (BoomRotation :type "Rotator Structure") (CameraOffset :type "Vector Structure") (CameraRotation :type "Rotator Structure") (CameraFOV :type "Float (double-precision)"))
  (set `self._BoomRotation` BoomRotation)
  (set `self._CameraOffset` CameraOffset)
  (set `self._CameraRotation` CameraRotation)
  (set `self._CameraFOV` CameraFOV)
  (`self.TransitionReset`)
  (bind _returnvalue (`KismetSystemLibrary.K2_SetTimerDelegate` (delegate `TransitionLoop`) 0.01 true))
  (set `self._TransitionTimer` _returnvalue))

(event `TransitionLoop`
  (if (> (`KismetSystemLibrary.GetGameTimeInSeconds`) 0.75)
    (if (not (and (`self._BoomDoneRotating`) (`self._CameraDoneRotating`) (`self._CameraDoneMoving`)))
      (`self.UpdateTime`)
      (`self._InterpBoomArmRotation` (`self._BoomRotation`))
      (`self._InterpCameraRotation` (`self._CameraRotation`))
      (`self._InterpCameraOffset` (`self._CameraOffset`))
      (`self._InterpCameraFOV` (`self._CameraFOV`))
      (else
        (`KismetSystemLibrary.K2_ClearAndInvalidateTimerHandle` (`self._TransitionTimer`))))))

(event `StartCameraShake`
  (params (ShakeClass :type "CameraShakeBase Class Reference"))
  (if (`KismetSystemLibrary.IsValidClass` ShakeClass)
    (if (!= (`GameplayStatics.GetObjectClass` (`self._CameraShake`)) ShakeClass)
      (`self.StopCameraShake`)
      (bind _returnvalue (`PlayerCameraManager.StartCameraShake` :`self` (`GameplayStatics.GetPlayerCameraManager` 0) :`ShakeClass` ShakeClass))
      (set `self._CameraShake` _returnvalue))))

(event `StopCameraShake`
  (bind __camerashake (`self._CameraShake`))
  (`/Engine/EditorBlueprintResources/StandardMacros.IsValid` __camerashake
    (:`Is Valid`
      (`PlayerCameraManager.StopCameraShake` (`GameplayStatics.GetPlayerCameraManager` 0) __camerashake true))))

(fn `_InterpBoomArmRotation`
  (params (Target :type "Rotator Structure"))
  (locals (LOC_Target :type "Rotator Structure"))
  (bind __ownerboom (`self._OwnerBoom`))
  (bind _output_get (set `local.LOC_Target` Target))
  (if (== _output_get (`SceneComponent.RelativeRotation` (`self._OwnerBoom`)) :`ErrorTolerance` 0.01)
    (set `self._BoomDoneRotating` true)
    (return)
    (else
      (`SceneComponent.K2_SetRelativeRotation` __ownerboom (`KismetMathLibrary.RInterpTo` (`SceneComponent.RelativeRotation` __ownerboom) (`local.LOC_Target`) (`self._Time`) (`self.TransitionSpeed`)) false false)
      (return))))

(fn `_InterpCameraFOV`
  (params (Target :type "Float (double-precision)"))
  (locals (LOC_Target :type "Float (double-precision)"))
  (bind _output_get (set `local.LOC_Target` Target))
  (if (`KismetMathLibrary.NearlyEqual_FloatFloat` _output_get (`CameraComponent.FieldOfView` (`self._OwnerCamera`)))
    (set `self._CameraDoneRotating` true)
    (return)
    (else
      (`CameraComponent.SetFieldOfView` (`self._OwnerCamera`) (`KismetMathLibrary.FInterpTo` (`CameraComponent.FieldOfView` (`self._OwnerCamera`)) (`local.LOC_Target`) (`self._Time`) (`self.TransitionSpeed`)))
      (return))))

(fn `_InterpCameraOffset`
  (params (Target :type "Vector Structure"))
  (locals (LOC_Target :type "Vector Structure"))
  (bind __ownercamera (`self._OwnerCamera`))
  (bind _output_get (set `local.LOC_Target` Target))
  (if (== _output_get (`SceneComponent.RelativeLocation` (`self._OwnerCamera`)) :`ErrorTolerance` 0.01)
    (set `self._CameraDoneMoving` true)
    (return)
    (else
      (`SceneComponent.K2_SetRelativeLocation` __ownercamera (`KismetMathLibrary.VInterpTo` (`SceneComponent.RelativeLocation` __ownercamera) (`local.LOC_Target`) (`self._Time`) (`self.TransitionSpeed`)) false false)
      (return))))

(fn `_InterpCameraRotation`
  (params (Target :type "Rotator Structure"))
  (locals (LOC_Target :type "Rotator Structure"))
  (bind __ownercamera (`self._OwnerCamera`))
  (bind _output_get (set `local.LOC_Target` Target))
  (if (== _output_get (`SceneComponent.RelativeRotation` (`self._OwnerCamera`)) :`ErrorTolerance` 0.01)
    (set `self._CameraDoneRotating` true)
    (return)
    (else
      (`SceneComponent.K2_SetRelativeRotation` __ownercamera (`KismetMathLibrary.RInterpTo` (`SceneComponent.RelativeRotation` __ownercamera) (`local.LOC_Target`) (`self._Time`) (`self.TransitionSpeed`)) false false)
      (return))))