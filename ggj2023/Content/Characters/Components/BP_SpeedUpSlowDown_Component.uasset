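; Hero movement component meant to speed up or slow down BP_HERO, still work in progress.
; On BeginPlay it caches the hero, its CharacterMovement and initial gravity scale.
; SlowDown overrides vertical velocity through LaunchCharacter, while SpeedUp only prints a not-working message.
; AdjustFallGravity scales the initial gravity and ResetGravity restores it, but the timed float and forward-launch logic is disconnected.
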(event `self.ReceiveBeginPlay`
  (bind _asbp_hero (cast `/Game/Characters/BP_HERO` (`self.GetOwner`))
    (:`then`
      (bind _output_get (set `self.As BP HERO Droplet` _asbp_hero))
      (set `self.As Character Movement` (`Character.CharacterMovement` _output_get))
      (set `self.InitialGravityScale` (`CharacterMovementComponent.GravityScale` (`self.As Character Movement`))))
    (:`CastFailed`
      (`KismetSystemLibrary.PrintString` "Error: Expecting HeroDroplet"))))

(event `SlowDown`
  (`Character.LaunchCharacter` (`self.As BP HERO Droplet`) (`KismetMathLibrary.MakeVector` 0.0 0.0 (`self.Slow_LaunchVelocityZ`)) false true))

(event `ResetFloat`
  (`KismetSystemLibrary.PrintString` "ResetFloat"))

(event `SpeedUp`
  (`KismetSystemLibrary.PrintString` "Speedup not quite wprking"))

(event `ResetGravity`
  (`KismetSystemLibrary.PrintString` "RESET")
  (`self.AdjustFallGravity` 1.0)
  (`KismetSystemLibrary.K2_ClearAndInvalidateTimerHandle` (`self.FloatTimer`)))

(fn `AdjustFallGravity`
  (params (GravityMultiple :type "Float (double-precision)"))
  (bind _as_character_movement (`self.As Character Movement`))
  (set `CharacterMovementComponent.GravityScale` (* GravityMultiple (`self.InitialGravityScale`)) (`self.As Character Movement`))
  (`KismetSystemLibrary.PrintString` (`KismetStringLibrary.Concat_StrStr` "Gravity Scale[" (`KismetStringLibrary.Conv_DoubleToString` (`CharacterMovementComponent.GravityScale` _as_character_movement)) "],  max walk speed[" (`KismetStringLibrary.Conv_DoubleToString` (`CharacterMovementComponent.MaxWalkSpeed` _as_character_movement)) "]")))

(fn `GetSlowDownMultiple`
  (returns (SlowDownMultiple :type "Float (single-precision)"))
  (return (`self.SlowDownMultiple`)))

(fn `SetSlowDownMultiple`
  (params (SlowDownMultiple :type "Float (single-precision)"))
  (set `self.SlowDownMultiple` SlowDownMultiple)
  (return))