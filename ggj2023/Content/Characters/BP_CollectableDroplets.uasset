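; BP_CollectableDroplets is a pooled droplet actor that can travel along splines and is spawned under a BP_RainPool owner.
; It caches that pool on BeginPlay and hands itself back through ReturntoPool, warning when no pool is assigned.
; Mesh hits are forwarded to its spline slide component.
; On spline release, it enables mesh physics with the exit velocity halved and reversed, logic marked as needing work.
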(event `self.ReceiveBeginPlay`
  (bind _asbp_rain_pool (cast `/Game/Blueprint/Rain/BP_RainPool` (`self.GetOwner`)))
  (set `self.As BP Rain Pool` _asbp_rain_pool))

(event `self.StaticMesh.OnComponentHit`
  (params (HitComponent :type "PrimitiveComponent Object Reference") (OtherActor :type "Actor Object Reference") (OtherComp :type "PrimitiveComponent Object Reference") (NormalImpulse :type "Vector Structure") (Hit :type "HitResult Structure (by ref)"))
  ;[0.1535 0 1] On HIT  / SPLINE object type
  (`/Game/Characters/Components/BP_SplineSlideComponent.Owner Collision Event` (`self.Bp_SplineSlideComponent`) OtherActor Hit null (`self.StaticMesh`)))

(event `/Game/Blueprint/Rain/BPI_RainPool.ReturnToPool`
  (bind _as_bp_rain_pool (`self.As BP Rain Pool`)
    (:`then`
      (`/Game/Blueprint/Rain/BP_RainPool.ReturnObjectToPool` _as_bp_rain_pool self))
    (:`else`
      (`KismetSystemLibrary.PrintString` "Warning: Calling Return to Pool on a Drop without an assigned Pool"))))

(event `self.BP_SplineSlideComponent.SplineReleasedActorEvent`
  (params (ExitVelocity :type "Vector Structure") (NewControlYaw :type "Float (double-precision)"))
  (`PrimitiveComponent.SetSimulatePhysics` (`self.StaticMesh`) true)
  (`PrimitiveComponent.SetPhysicsLinearVelocity` (`self.StaticMesh`) (* ExitVelocity -0.5) false "None"))

(fn `UserConstructionScript`)