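; BP_RootsGameInstance is the game instance that manages background music across level transitions.
; Its ChangeMusic event crossfades tracks by fading out the current one, then spawning a persistent 2D sound that fades in and becomes current.
; Helper functions for title, win, lose and level music call it with a default transition time and either menu or level volume.
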(event `ChangeMusic`
  (params (NewMusic :type "SoundBase Object Reference") (TransitionTime :type "Float (single-precision)") (VolumeMultiplier :type "Float (single-precision)"))
  (bind _currentmusic (`self.CurrentMusic`))
  (`/Engine/EditorBlueprintResources/StandardMacros.IsValid` _currentmusic
    (:`Is Valid`
      (bind _output_get (set `self.PreviousMusic` _currentmusic))
      (`AudioComponent.FadeOut` _output_get TransitionTime 0.0 "Linear"))
    (:`Is Not Valid`
      _))
  (bind _returnvalue (`GameplayStatics.SpawnSound2D` NewMusic VolumeMultiplier 1.0 0.0 null true))
  (bind _output_get_2 (set `self.CurrentMusic` _returnvalue))
  (`AudioComponent.FadeIn` _output_get_2 TransitionTime 1.0 0.0 "Linear"))

(fn `PlayLevelMusic`
  (`self.ChangeMusic` (`self.LevelMusic`) (`self.DefaultTransitionTime`) (`self.LevelVolume`)))

(fn `PlayLoseMusic`
  (`self.ChangeMusic` (`self.LoseMusic`) (`self.DefaultTransitionTime`) (`self.MenuVolume`)))

(fn `PlayTitleMusic`
  (`self.ChangeMusic` (`self.TitleMusic`) (`self.DefaultTransitionTime`) (`self.MenuVolume`)))

(fn `PlayWinMusic`
  (`self.ChangeMusic` (`self.WinMusic`) (`self.DefaultTransitionTime`) (`self.MenuVolume`)))