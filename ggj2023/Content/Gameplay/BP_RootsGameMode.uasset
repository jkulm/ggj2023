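; BP_RootsGameMode is the game mode that handles the end of a match, showing a win or lose screen.
; FinishGame pauses the game, then creates and adds WBP_WinMenu or WBP_LoseMenu to the viewport based on the Won flag.
; It then has BP_RootsGameInstance play the matching win or lose music.
; The event graph and construction script hold no logic.
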(fn `FinishGame`
  (params (Won :type Boolean))
  (bind _returnvalue (`GameplayStatics.GetGameInstance`))
  (bind _returnvalue_2 (`GameplayStatics.GetPlayerController` 0))
  (`GameplayStatics.SetGamePaused` true)
  (if Won
    (bind _returnvalue_3 (`|CreateWidget` "/Game/UI/Menus/WBP_WinMenu.WBP_WinMenu_C" _returnvalue_2))
    (`UserWidget.AddToViewport` _returnvalue_3 0)
    (bind _asbp_roots_game_instance (cast `/Game/Gameplay/BP_RootsGameInstance` _returnvalue))
    (`/Game/Gameplay/BP_RootsGameInstance.PlayWinMusic` _asbp_roots_game_instance)
    (else
      (bind _returnvalue_4 (`|CreateWidget` "/Game/UI/Menus/WBP_LoseMenu.WBP_LoseMenu_C" _returnvalue_2))
      (`UserWidget.AddToViewport` _returnvalue_4 0)
      (bind _asbp_roots_game_instance_2 (cast `/Game/Gameplay/BP_RootsGameInstance` _returnvalue))
      (`/Game/Gameplay/BP_RootsGameInstance.PlayLoseMusic` _asbp_roots_game_instance_2))))

(fn `UserConstructionScript`)